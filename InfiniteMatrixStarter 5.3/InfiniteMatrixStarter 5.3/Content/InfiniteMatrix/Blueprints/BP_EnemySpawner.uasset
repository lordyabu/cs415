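; BP_EnemySpawner spawns BP_Enemy actors at randomized positions, starting with one on BeginPlay.
; SpawnEnemy stores each new enemy as NewestEnemy and gives it a reference back to the spawner.
; SpawnEnemyAtSpawnPoint, not called here, places the next enemy at a random X offset from the newest one's SpawnPoint.
; It then sphere-checks randomized positions, looping on overlap to destroy an existing enemy and spawn another without that offset.
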(event `self.ReceiveBeginPlay`
  (`self.SpawnEnemy` (`KismetMathLibrary.MakeVector` 2000.0 (`KismetMathLibrary.Conv_IntToDouble` (`KismetMathLibrary.RandomIntegerInRange` -100 100)) (`KismetMathLibrary.Conv_IntToDouble` (`KismetMathLibrary.RandomIntegerInRange` -100 100)))))

(fn `SpawnEnemy`
  (params (`Spawn Transform Location` :type "Vector Structure"))
  (bind _returnvalue (`|SpawnActorFromClass` "/Game/InfiniteMatrix/Blueprints/BP_Enemy.BP_Enemy_C" (`KismetMathLibrary.MakeTransform` `Spawn Transform Location`) "Undefined" "MultiplyWithRoot" null null))
  (bind _output_get (set `self.NewestEnemy` _returnvalue))
  (set `/Game/InfiniteMatrix/Blueprints/BP_Enemy.EnemySpawner` self _output_get))

(fn `SpawnEnemyAtSpawnPoint`
  (bind _returnvalue (`KismetMathLibrary.RandomFloatInRange` 150.0 350.0))
  (bind _returnvalue_2 (`KismetMathLibrary.RandomFloatInRange` 0.0 20000.0))
  (bind _returnvalue_3 (`KismetMathLibrary.RandomFloatInRange` -150.0 250.0))
  (bind _returnvalue_4 (`KismetMathLibrary.RandomFloatInRange` 150.0 350.0))
  (bind _returnvalue_5 (`KismetMathLibrary.RandomFloatInRange` -150.0 250.0))
  (bind _returnvalue_x (`KismetMathLibrary.BreakVector` (`SceneComponent.K2_GetComponentLocation` (`/Game/InfiniteMatrix/Blueprints/BP_Enemy.SpawnPoint` (`self.NewestEnemy`)))))
  (bind _returnvalue_6 (+ _returnvalue_2 _returnvalue_x))
  (`self.SpawnEnemy` (`KismetMathLibrary.MakeVector` _returnvalue_6 _returnvalue_5 _returnvalue_4))
  (`KismetSystemLibrary.SphereOverlapActors` (`KismetMathLibrary.MakeVector` _returnvalue_6 _returnvalue_5 _returnvalue_4) 50.0 (`self.Object Types`))
  (while (stale _returnvalue_7) :!label _label
    (bind _outactors (`GameplayStatics.GetAllActorsOfClass` "/Game/InfiniteMatrix/Blueprints/BP_Enemy.BP_Enemy_C"))
    (for _array_element _outactors
      (`self.K2_DestroyActor` _array_element)
      (`self.SpawnEnemy` (`KismetMathLibrary.MakeVector` _returnvalue_2 _returnvalue_3 _returnvalue))
      (bind (_outactors_2 _returnvalue_7) (`KismetSystemLibrary.SphereOverlapActors` (`KismetMathLibrary.MakeVector` _returnvalue_2 _returnvalue_3 _returnvalue) 50.0 (`self.Object Types`)))
      (goto _label))))

(fn `UserConstructionScript`)