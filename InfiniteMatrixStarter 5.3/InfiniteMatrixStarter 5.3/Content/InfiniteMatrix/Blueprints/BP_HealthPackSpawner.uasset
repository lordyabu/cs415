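; Spawner actor that places BP_HealthPack pickups at random positions along the X axis, starting with one on BeginPlay.
; SpawnHealthPack stores the newest pack and passes it a reference to the spawner.
; SpawnHealthPackAtSpawnPoint, not called here, spawns the next pack at a random X offset from the newest pack's SpawnPoint.
; It then sphere-checks a separately randomized point, and while that finds packs, destroys one from all existing packs, respawns and rechecks.
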(event `self.ReceiveBeginPlay`
  (`self.SpawnHealthPack` (`KismetMathLibrary.MakeVector` (`KismetMathLibrary.RandomFloatInRange` 2000.0 4000.0) (`KismetMathLibrary.RandomFloatInRange` -300.0 400.0) (`KismetMathLibrary.RandomFloatInRange` 0.0 500.0))))

(fn `SpawnHealthPack`
  (params (`Spawn Location` :type "Vector Structure"))
  (bind _returnvalue (`|SpawnActorFromClass` "/Game/InfiniteMatrix/Blueprints/BP_HealthPack.BP_HealthPack_C" (`KismetMathLibrary.MakeTransform` `Spawn Location`) "Undefined" "MultiplyWithRoot" null null))
  (bind _output_get (set `self.NewestHealthPack` _returnvalue))
  (set `/Game/InfiniteMatrix/Blueprints/BP_HealthPack.HealthPackSpawner` self _output_get))

(fn `SpawnHealthPackAtSpawnPoint`
  (bind _returnvalue (`KismetMathLibrary.RandomFloatInRange` 0.0 500.0))
  (bind _returnvalue_2 (`KismetMathLibrary.RandomFloatInRange` -300.0 400.0))
  (bind _returnvalue_3 (`KismetMathLibrary.RandomFloatInRange` 0.0 500.0))
  (bind _returnvalue_4 (`KismetMathLibrary.RandomFloatInRange` -300.0 400.0))
  (bind _returnvalue_x (`KismetMathLibrary.BreakVector` (`SceneComponent.K2_GetComponentLocation` (`/Game/InfiniteMatrix/Blueprints/BP_HealthPack.SpawnPoint` (`self.NewestHealthPack`)))))
  (bind _returnvalue_5 (+ (`KismetMathLibrary.RandomFloatInRange` 0.0 20000.0) _returnvalue_x))
  (`self.SpawnHealthPack` (`KismetMathLibrary.MakeVector` _returnvalue_5 _returnvalue_4 _returnvalue_3))
  (`KismetSystemLibrary.SphereOverlapActors` (`KismetMathLibrary.MakeVector` _returnvalue_5 _returnvalue_4 _returnvalue_3) 50.0 (`self.Object Types`) "/Game/InfiniteMatrix/Blueprints/BP_HealthPack.BP_HealthPack_C")
  (while (stale _returnvalue_6) :!label _label
    (bind _outactors (`GameplayStatics.GetAllActorsOfClass` "/Game/InfiniteMatrix/Blueprints/BP_HealthPack.BP_HealthPack_C"))
    (for _array_element _outactors
      (`self.K2_DestroyActor` _array_element)
      (`self.SpawnHealthPack` (`KismetMathLibrary.MakeVector` _returnvalue_5 _returnvalue_2 _returnvalue))
      (bind (_outactors_2 _returnvalue_6) (`KismetSystemLibrary.SphereOverlapActors` (`KismetMathLibrary.MakeVector` _returnvalue_5 _returnvalue_2 _returnvalue) 50.0 (`self.Object Types`) "/Game/InfiniteMatrix/Blueprints/BP_HealthPack.BP_HealthPack_C"))
      (goto _label))))

(fn `UserConstructionScript`)